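; AI follower character that chases the player on detection and blows up on contact, spawning a radial-force projectile and destroying itself.
; Sphere overlap with the FirstPersonCharacter sets a follow flag, cleared on exit or after ten seconds.
; Tick moves toward the player while following, otherwise, after a delay, to a random reachable point around a MoveIa actor captured by Sphere1's hit event.
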(event `self.ReceiveHit`
  (params (MyComp :type "PrimitiveComponent Object Reference") (Other :type "Actor Object Reference") (OtherComp :type "PrimitiveComponent Object Reference") (bSelfMoved :type Boolean) (HitLocation :type "Vector Structure") (HitNormal :type "Vector Structure") (NormalImpulse :type "Vector Structure") (Hit :type "HitResult Structure (by ref)"))
  (cast `/Game/FirstPersonBP/Blueprints/FirstPersonCharacter` Other)
  (`|SpawnActorFromClass` "/Game/FirstPersonBP/Blueprints/RadialForce_Projectil_positif.RadialForce_Projectil_positif_C" (`self.GetTransform`) "Undefined" "OverrideRootScale")
  (`self.K2_DestroyActor`))

(event `self.Sphere.OnComponentEndOverlap`
  (params (OtherActor :type "Actor Object Reference") (OtherComp :type "PrimitiveComponent Object Reference") (OtherBodyIndex :type Integer))
  (cast `/Game/FirstPersonBP/Blueprints/FirstPersonCharacter` OtherActor)
  (set `self.varfollow` false))

(event `self.Sphere.OnComponentBeginOverlap`
  (params (OtherActor :type "Actor Object Reference") (OtherComp :type "PrimitiveComponent Object Reference") (OtherBodyIndex :type Integer) (bFromSweep :type Boolean) (SweepResult :type "HitResult Structure (by ref)"))
  (cast `/Game/FirstPersonBP/Blueprints/FirstPersonCharacter` OtherActor)
  (set `self.varfollow` true)
  (`KismetSystemLibrary.Delay` 10.0)
  (set `self.varfollow` false))

(event `self.ReceiveTick`
  (params (DeltaSeconds :type "Float (single-precision)"))
  (bind _returnvalue (`self.GetController`))
  (if (`self.varfollow`)
    (`NavigationSystem.SimpleMoveToActor` _returnvalue (`GameplayStatics.GetPlayerCharacter` 0))
    (else
      (`KismetSystemLibrary.Delay` 2.0)
      (`NavigationSystem.SimpleMoveToLocation` _returnvalue (`NavigationSystem.GetRandomReachablePointInRadius` (`self.K2_GetActorLocation` (stale `self.Sphere1.OnComponentHit` _asmove_ia)) 2000.0)))))

(event `self.Sphere1.OnComponentHit`
  (params (OtherActor :type "Actor Object Reference") (OtherComp :type "PrimitiveComponent Object Reference") (NormalImpulse :type "Vector Structure") (Hit :type "HitResult Structure (by ref)"))
  (bind _asmove_ia (cast `/Game/Blueprints/MoveIa` OtherActor)))

(fn `UserConstructionScript`)