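; A cube actor with magnet-like polarity: positive and negative projectile hits set its charge, and other hits raise a one-second stop flag.
; When charged, a sphere overlap with a "nega" or "posi" tagged actor drives MoveComponentTo on the mesh, or stops it while flagged.
; Both charges target the impact point for "nega" and a mirrored point away for "posi", so they attract and repel identically.
; An older hit-based movement chain is left unconnected.
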(event `self.ReceiveTick`
  (params (DeltaSeconds :type "Float (single-precision)")))

(event `self.ReceiveBeginPlay`
  (set `self.varpositf` false))

(event `self.ReceiveHit`
  (params (MyComp :type "PrimitiveComponent Object Reference") (Other :type "Actor Object Reference") (OtherComp :type "PrimitiveComponent Object Reference") (bSelfMoved :type Boolean) (HitLocation :type "Vector Structure") (HitNormal :type "Vector Structure") (NormalImpulse :type "Vector Structure") (Hit :type "HitResult Structure (by ref)"))
  (if (`self.varpositf`)
    (cast `/Game/FirstPersonBP/Blueprints/Projectil_negatif` Other :!label _label
      (:`then`
        (set `self.varnegatif` true)
        (set `self.varpositf` false))
      (:`CastFailed`
        (set `self.varEndmove` true)
        (`KismetSystemLibrary.Delay` 1.0)
        (set `self.varEndmove` false)))
    (else
      (cast `/Game/FirstPersonBP/Blueprints/Projectil_positif` Other
        (:`then`
          (set `self.varpositf` true)
          (set `self.varnegatif` false))
        (:`CastFailed`
          (goto _label))))))

(event `self.Sphere.OnComponentBeginOverlap`
  (params (OtherActor :type "Actor Object Reference") (OtherComp :type "PrimitiveComponent Object Reference") (OtherBodyIndex :type Integer) (bFromSweep :type Boolean) (SweepResult :type "HitResult Structure (by ref)"))
  (bind (_bblockinghit _binitialoverlap _time _location _impactpoint) (`GameplayStatics.BreakHitResult` SweepResult))
  (bind _returnvalue (`self.ActorHasTag` OtherActor "nega"))
  (bind _returnvalue_2 (`self.ActorHasTag` OtherActor "posi"))
  (bind _vectorentre (`self.vectorentre`))
  (bind _returnvalue_3 (`KismetMathLibrary.MakeVector` (.x (- _impactpoint (+ _vectorentre _vectorentre))) (.y (- _impactpoint (+ _vectorentre _vectorentre))) (.z (`self.K2_GetActorLocation`))))
  (set `self.vectorentre` (- _impactpoint (`self.K2_GetActorLocation`)))
  (if (`self.varpositf`)
    ;[1 1 1] positif cube
    (if _returnvalue
      ;;[1 1 1] negatif object overlaps
      (if (`self.varEndmove`)
        (goto _label_2 :!via `Stop`)
        (else
          (`KismetSystemLibrary.MoveComponentTo` (`self.StaticMeshComponent`) _impactpoint (struct) false false 0.5 :!label _label_2)))
      (elif _returnvalue_2
        ;;[1 1 1] positif object overlaps
        (if (`self.varEndmove`)
          (goto _label_3 :!via `Stop`)
          (else
            (`KismetSystemLibrary.MoveComponentTo` (`self.StaticMeshComponent`) _returnvalue_3 :!label _label_3)))))
    (elif (`self.varnegatif`)
      ;[1 1 1] negatif cube
      (if _returnvalue
        ;;[1 1 1] positif object overlaps
        (if (`self.varEndmove`)
          (goto _label_4 :!via `Stop`)
          (else
            (`KismetSystemLibrary.MoveComponentTo` (`self.StaticMeshComponent`) _impactpoint :!label _label_4)))
        (else
          ;;[1 1 1] negatif object overlap
          (if _returnvalue_2
            (if (`self.varEndmove`)
              (goto _label_5 :!via `Stop`)
              (else
                (`KismetSystemLibrary.MoveComponentTo` (`self.StaticMeshComponent`) _returnvalue_3 (struct) false false 0.5 :!label _label_5)))))))))

(fn `UserConstructionScript`)