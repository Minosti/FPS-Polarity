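; Tourelle (turret) Blueprint that fires a homing-style projectile when a first-person character enters its detection sphere.
; On Sphere begin overlap, it spawns one Projectile at the Billboard's location and sets its ProjectilTarget to the character's capsule component.
; There is no timer or repeat fire, so each entry yields a single shot.
; The end overlap handler on Sphere1 only casts to the character and has no further effect.
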(event `self.Sphere.OnComponentBeginOverlap`
  (params (OtherActor :type "Actor Object Reference") (OtherComp :type "PrimitiveComponent Object Reference") (OtherBodyIndex :type Integer) (bFromSweep :type Boolean) (SweepResult :type "HitResult Structure (by ref)"))
  (bind _asfirst_person_character (cast `/Game/FirstPersonBP/Blueprints/FirstPersonCharacter` OtherActor))
  (set `self.Target` (`Character.CapsuleComponent` _asfirst_person_character))
  (bind _returnvalue (`|SpawnActorFromClass` "/Game/Blueprints/projectile.projectile_C" (`KismetMathLibrary.Conv_VectorToTransform` (`SceneComponent.K2_GetComponentLocation` (`self.Billboard`))) "Undefined" "OverrideRootScale"))
  (set `/Game/Blueprints/projectile.projectil target` (`self.Target`) _returnvalue))

(event `self.Sphere1.OnComponentEndOverlap`
  (params (OtherActor :type "Actor Object Reference") (OtherComp :type "PrimitiveComponent Object Reference") (OtherBodyIndex :type Integer))
  (cast `/Game/FirstPersonBP/Blueprints/FirstPersonCharacter` OtherActor))

(fn `UserConstructionScript`)