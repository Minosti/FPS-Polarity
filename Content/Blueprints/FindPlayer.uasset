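; Behavior tree task that checks whether the player is within the perception radius of an AI_Follower_Cours controller.
; It compares the horizontal distance between the player character and the owner actor to the controller's PerceptionRadius.
; When in range, it writes the player's location to the PlayerPosition blackboard key and succeeds.
; It fails when out of range or when the controller cast fails.
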(event `self.ReceiveExecute`
  (params (OwnerActor :type "Actor Object Reference"))
  (bind _returnvalue (`GameplayStatics.GetPlayerCharacter` 0))
  (bind _returnvalue_2 (`AIBlueprintHelperLibrary.GetAIController` OwnerActor))
  (bind _asai_follower_cours (cast `/Game/Blueprints/AI_Follower_Cours` _returnvalue_2)
    (:`then`
      (`|ExecutionSequence`
        (:`then_0`
          (bind _returnvalue_3 (<= (`Actor.GetHorizontalDistanceTo` _returnvalue OwnerActor) (`/Game/Blueprints/AI_Follower_Cours.PerceptionRadius` _asai_follower_cours)))
          (if _returnvalue_3
            (`BTFunctionLibrary.SetBlackboardValueAsVector` (`self.Player Position`) (`Actor.K2_GetActorLocation` _returnvalue))))
        (:`then_1`
          (`self.FinishExecute` _returnvalue_3))))
    (:`CastFailed`
      (`self.FinishExecute` false))))